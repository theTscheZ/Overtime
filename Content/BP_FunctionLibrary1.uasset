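; Blueprint function library with a case-insensitive string comparison that returns whether string A sorts before string B.
; It lowercases both strings, then compares character codes up to the shorter length, returning at the first difference.
; When the shared prefix matches, the shorter string counts as less, and equal strings return false.
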(fn `Is String A Less Than String B`
  (params (A :type String) (B :type String))
  (returns (Result :type Boolean))
  (locals (LocalA :type String) (LocalB :type String) (LocalArrayA :type "Array of String") (LocalArrayB :type "Array of String") (LocalLengthA :type Integer) (LocalLengthB :type Integer) (Count :type Integer))
  (bind _locallengtha (`local.LocalLengthA`))
  (bind _locallengthb (`local.LocalLengthB`))
  (`|ExecutionSequence`
    (:`then_0`
      ;[0 0.05118 1] Convert each string to lower case and store as an array of characters
      (bind _output_get (set `local.LocalA` (`KismetStringLibrary.ToLower` A)))
      (set `local.LocalArrayA` (`KismetStringLibrary.GetCharacterArrayFromString` _output_get)))
    (:`then_1`
      (bind _output_get_2 (set `local.LocalB` (`KismetStringLibrary.ToLower` B)))
      (set `local.LocalArrayB` (`KismetStringLibrary.GetCharacterArrayFromString` _output_get_2)))
    (:`then_2`
      ;[0 1 0.004274] Get the length of each string
      (set `local.LocalLengthA` (`KismetArrayLibrary.Array_Length` (`local.LocalArrayA`)))
      (set `local.LocalLengthB` (`KismetArrayLibrary.Array_Length` (`local.LocalArrayB`))))
    (:`then_3`
      ;[0.9427 1 0] Determine the number of iterations of the next FOR LOOP (the length of whichever string is shorter)
      (if (<= (`local.LocalLengthA`) (`local.LocalLengthB`))
        (set `local.Count` (`local.LocalLengthA`))
        (else
          (set `local.Count` (`local.LocalLengthB`)))))
    (:`then_4`
      ;[1 0 0.0222] For each character convert it to its ascii number and compare the numbers
      (bind _result (`/Engine/EditorBlueprintResources/StandardMacros.DecrementInt` (`local.Count`))
        (:`  `
          (for _index (range (+ _result 1))
            (if (< (`KismetStringLibrary.GetCharacterAsNumber` (`local.LocalA`) _index) (`KismetStringLibrary.GetCharacterAsNumber` (`local.LocalB`) _index))
              (return true)
              (elif (not (== (`KismetStringLibrary.GetCharacterAsNumber` (`local.LocalA`) _index) (`KismetStringLibrary.GetCharacterAsNumber` (`local.LocalB`) _index)))
                (return false))))
          (if (== _locallengtha _locallengthb)
            (return false) ; Strings are equal
            (elif (< _locallengtha _locallengthb)
              (return true) ; StringA is less than StringB
              (else
                (return false) ; StringA is greater than StringB
              ))))))))