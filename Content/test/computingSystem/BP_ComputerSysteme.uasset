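; BP_ComputerSysteme is an interactable computer that the player can enter and leave through a menu screen.
; OnInteract alternates via FlipFlop: first blending the view to the computer, then, after the blend delay, showing WBP_PC_MainMenu with cursor and Game-and-UI input.
; The next interaction blends back to BP_FirstPersonCharacter, removes the widget and hides the cursor, without resetting input mode.
; The camera target comes from GetActorOfClass rather than self, so it assumes one computer per level.
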(event `/Game/Tasks/Interfaces/BPI_Interactable.OnInteract`
  (params (InteractingPlayer :type "/Game/FirstPerson/Blueprints/BP_FirstPersonCharacter Object Reference"))
  (bind _returnvalue (`GameplayStatics.GetPlayerController` 0))
  (`/Engine/EditorBlueprintResources/StandardMacros.FlipFlop`
    (:`A`
      (`self.ChangeCam`)
      (`KismetSystemLibrary.Delay` (`self.Blend Time`))
      (bind _returnvalue_2 (`|CreateWidget` "/Game/test/computingSystem/WBP_PC_MainMenu.WBP_PC_MainMenu_C" (`GameplayStatics.GetPlayerController` 0)))
      (`UserWidget.AddToViewport` _returnvalue_2 0)
      (set `PlayerController.bShowMouseCursor` true _returnvalue)
      (`WidgetBlueprintLibrary.SetInputMode_GameAndUIEx` (`GameplayStatics.GetPlayerController` 0) _returnvalue_2 "DoNotLock" false))
    (:`B`
      (`self.ChangeCamBack`)
      (`Widget.RemoveFromParent` _returnvalue_2)
      (set `PlayerController.bShowMouseCursor` false _returnvalue))))

(fn `ChangeCam`
  (cast `/Game/FirstPerson/Blueprints/BP_FirstPersonCharacter` (`GameplayStatics.GetPlayerCharacter` 0))
  (bind _returnvalue (`GameplayStatics.GetActorOfClass` "BP_ComputerSysteme_C"))
  (`PlayerController.SetViewTargetWithBlend` (`GameplayStatics.GetPlayerController` 0) _returnvalue (`self.Blend Time`) "VTBlend_Linear" 0.0 false))

(fn `ChangeCamBack`
  (bind _asbp_first_person_character (cast `/Game/FirstPerson/Blueprints/BP_FirstPersonCharacter` (`GameplayStatics.GetPlayerCharacter` 0)))
  (`PlayerController.SetViewTargetWithBlend` (`GameplayStatics.GetPlayerController` 0) _asbp_first_person_character 0.35 "VTBlend_Cubic" 0.0 false))

(fn `UserConstructionScript`)