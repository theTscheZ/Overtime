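; Game state that manages sanity, day progression and the "save1" save slot.
; On BeginPlay it loads or creates the save, restores progress and display settings, activates tasks and starts the HUD and timer.
; A one-second timer drains sanity down to the current day's floor, and threshold checks swap the HUD's match material.
; ChangeDay stops the timer, lowers that floor, saves and reopens FirstPersonMap.
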(event `self.ReceiveBeginPlay`
  (`KismetSystemLibrary.DelayUntilNextTick`)
  (`|ExecutionSequence`
    (:`then_0`
      (`self.SetSanityLevels`))
    (:`then_1`
      (bind _returnvalue (`GameplayStatics.GetActorOfClass` "/Script/Engine.PostProcessVolume"))
      (set `self.PPV` _returnvalue))
    (:`then_2`
      (bind _returnvalue_2 (`GameplayStatics.DoesSaveGameExist` "save1 "))
      (if _returnvalue_2
        (bind _returnvalue_3 (`GameplayStatics.LoadGameFromSlot` "save1 "))
        (bind _asbp_save_game (cast `/Game/SaveGame/BP_SaveGame` _returnvalue_3))
        (bind _output_get (set `self.BP Save` _asbp_save_game))
        (`self.RestoreSave` _output_get)
        (`KismetSystemLibrary.PrintString` "loaded")
        (else
          (`KismetSystemLibrary.PrintString` "create")
          (bind _returnvalue_4 (`GameplayStatics.CreateSaveGameObject` "/Game/SaveGame/BP_SaveGame.BP_SaveGame_C"))
          (set `self.BP Save` _returnvalue_4)
          (set `self.Sanity` (`self.MaxSanity`))
          (set `self.SanityLimit` (`KismetMathLibrary.Conv_IntToDouble` (`self.Sanity90`)))
          (`self.ConfigureSave`)
          (`GameplayStatics.SaveGameToSlot` _returnvalue_4 "save1 ")))
      (`self.GetHUD`)
      (`self.ActivateTasks`))))

(event `Change Day`
  (params (`Current Day` :type Integer))
  (if (`KismetSystemLibrary.K2_IsValidTimerHandle` (`self.Timer`))
    (`self.StopTimer`))
  (switch `int` `Current Day`
    (:`1`
      (bind _output_get (set `self.SanityLimit` (`KismetMathLibrary.Conv_IntToDouble` (`self.Sanity70`))))
      (`KismetSystemLibrary.PrintString` (`KismetStringLibrary.Conv_DoubleToString` _output_get)))
    (:`2`
      (bind _output_get_2 (set `self.SanityLimit` (`KismetMathLibrary.Conv_IntToDouble` (`self.Sanity50`))))
      (`KismetSystemLibrary.PrintString` (`KismetStringLibrary.Conv_DoubleToString` _output_get_2)))
    (:`3`
      (bind _output_get_3 (set `self.SanityLimit` (`KismetMathLibrary.Conv_IntToDouble` (`self.Sanity30`))))
      (`KismetSystemLibrary.PrintString` (`KismetStringLibrary.Conv_DoubleToString` _output_get_3)))
    (:`4`
      (bind _output_get_4 (set `self.SanityLimit` 0.0))
      (`KismetSystemLibrary.PrintString` (`KismetStringLibrary.Conv_DoubleToString` _output_get_4))))
  (bind _returnvalue (`GameplayStatics.DoesSaveGameExist` "save1 "))
  (if _returnvalue
    (`self.ConfigureSave`)
    (bind _returnvalue_2 (`GameplayStatics.SaveGameToSlot` (`self.BP Save`) "save1 "))
    (`KismetSystemLibrary.PrintString` "saved" _returnvalue_2)
    (`GameplayStatics.OpenLevel` "FirstPersonMap")
    (else
      (`KismetSystemLibrary.PrintString` "no save"))))

(event `StartTimer`
  (bind _returnvalue (`KismetSystemLibrary.K2_SetTimerDelegate` (delegate `Count`) 1.0 true))
  (set `self.Timer` _returnvalue))

(event `Count`
  (if (> (`self.Sanity`) (`self.SanityLimit`))
    (bind _result (`/Engine/EditorBlueprintResources/StandardMacros.DecrementFloat` (`self.Sanity`))
      (:`  `
        (`KismetSystemLibrary.PrintString` (`KismetStringLibrary.Conv_DoubleToString` _result))
        (`self.RefreshMat`)))))

(event `StopTimer`
  (`KismetSystemLibrary.K2_PauseTimerHandle` (`self.Timer`)))

(event `GetHUD`
  (bind _foundwidgets (`WidgetBlueprintLibrary.GetAllWidgetsOfClass` "/Game/FirstPerson/Blueprints/W_MainHUD.W_MainHUD_C"))
  (bind _output_get (set `self.HUD` (`|GetArrayItem` _foundwidgets)))
  (`/Engine/EditorBlueprintResources/StandardMacros.IsValid` _output_get
    (:`Is Valid`
      (`Widget.SetVisibility` (`self.HUD`) "Visible")
      (`self.RefreshMat`)
      (`self.StartTimer`))
    (:`Is Not Valid`
      (`KismetSystemLibrary.PrintString` "wtf"))))

(event `RefreshMat`
  (`self.CheckSanity` (`KismetMathLibrary.FTrunc` (`self.Sanity`)))
  (`KismetSystemLibrary.PrintString` (`KismetStringLibrary.Conv_IntToString` (`self.CurrentDay`))))

(fn `AddSanity`
  (params (SanityToAdd :type "Float (double-precision)"))
  (bind _returnvalue (+ SanityToAdd (`self.Sanity`)))
  (if (> _returnvalue (`self.MaxSanity`))
    (set `self.Sanity` (`self.MaxSanity`))
    (else
      (set `self.Sanity` _returnvalue)))
  (`self.RefreshMat`))

(fn `CheckSanity`
  (params (Sanity :type Integer))
  (if (> Sanity (`self.Sanity90`))
    (`/Game/FirstPerson/Blueprints/W_MainHUD.Change_Match_State` (`self.HUD`) "/Game/Menu/Streichholz/100_anim_sprites_Mat.100_anim_sprites_Mat")
    (elif (> Sanity (`self.Sanity80`))
      (`/Game/FirstPerson/Blueprints/W_MainHUD.Change_Match_State` (`self.HUD`) "/Game/Menu/Streichholz/90_anim_sprites_Mat.90_anim_sprites_Mat")
      (elif (> Sanity (`self.Sanity70`))
        (`/Game/FirstPerson/Blueprints/W_MainHUD.Change_Match_State` (`self.HUD`) "/Game/Menu/Streichholz/80_anim_sprites_Mat.80_anim_sprites_Mat")
        (elif (> Sanity (`self.Sanity60`))
          (`/Game/FirstPerson/Blueprints/W_MainHUD.Change_Match_State` (`self.HUD`) "/Game/Menu/Streichholz/70_anim_sprites_Mat.70_anim_sprites_Mat")
          (elif (> Sanity (`self.Sanity50`))
            (`/Game/FirstPerson/Blueprints/W_MainHUD.Change_Match_State` (`self.HUD`) "/Game/Menu/Streichholz/60_anim_sprites_Mat.60_anim_sprites_Mat")
            (elif (> Sanity (`self.Sanity40`))
              (`/Game/FirstPerson/Blueprints/W_MainHUD.Change_Match_State` (`self.HUD`) "/Game/Menu/Streichholz/50_anim_sprites_Mat.50_anim_sprites_Mat")
              (elif (> Sanity (`self.Sanity30`))
                (`/Game/FirstPerson/Blueprints/W_MainHUD.Change_Match_State` (`self.HUD`) "/Game/Menu/Streichholz/40_anim_sprites_Mat.40_anim_sprites_Mat")
                (elif (> Sanity (`self.Sanity20`))
                  (`/Game/FirstPerson/Blueprints/W_MainHUD.Change_Match_State` (`self.HUD`) "/Game/Menu/Streichholz/30_anim_sprites_Mat.30_anim_sprites_Mat")
                  (elif (> Sanity (`self.Sanity10`))
                    (`/Game/FirstPerson/Blueprints/W_MainHUD.Change_Match_State` (`self.HUD`) "/Game/Menu/Streichholz/20_anim_sprites_Mat.20_anim_sprites_Mat")
                    (elif (> Sanity 0)
                      (`/Game/FirstPerson/Blueprints/W_MainHUD.Change_Match_State` (`self.HUD`) "/Game/Menu/Streichholz/10_anim_sprites_Mat.10_anim_sprites_Mat")
                      (else
                        (`/Game/FirstPerson/Blueprints/W_MainHUD.Change_Match_State` (`self.HUD`) "/Game/Menu/Streichholz/0_Mat.0_Mat")))))))))))))

(fn `ConfigureSave`
  (bind _bp_save (`self.BP Save`))
  (`|ExecutionSequence`
    (:`then_0`
      (set `/Game/SaveGame/BP_SaveGame.Sanity` (`self.Sanity`) _bp_save)
      (set `/Game/SaveGame/BP_SaveGame.SanityLimit` (`self.SanityLimit`) _bp_save)
      (set `/Game/SaveGame/BP_SaveGame.CurrentDay` (`self.CurrentDay`) _bp_save))
    (:`then_1`
      (set `/Game/SaveGame/BP_SaveGame.Brightness` (`self.Brightness`) _bp_save)
      (set `/Game/SaveGame/BP_SaveGame.Contrast` (`self.Contrast`) _bp_save)
      (set `/Game/SaveGame/BP_SaveGame.FOV` (`self.FOV`) _bp_save))))

(fn `RestoreSave`
  (params (`BP Save` :type "/Game/SaveGame/BP_SaveGame Object Reference"))
  (bind _contrast (`/Game/SaveGame/BP_SaveGame.Contrast` `BP Save`))
  (bind _returnvalue (* (`/Game/SaveGame/BP_SaveGame.Brightness` `BP Save`) -1.0))
  (`|ExecutionSequence`
    (:`then_0`
      (set `self.CurrentDay` (`/Game/SaveGame/BP_SaveGame.CurrentDay` `BP Save`))
      (set `self.Sanity` (`/Game/SaveGame/BP_SaveGame.Sanity` `BP Save`))
      (set `self.SanityLimit` (`/Game/SaveGame/BP_SaveGame.SanityLimit` `BP Save`)))
    (:`then_1`
      (setmembers `PostProcessSettings` :`StructRef` (`PostProcessVolume.Settings` (`self.PPV`)) :`AutoExposureMinBrightness` _returnvalue :`AutoExposureMaxBrightness` _returnvalue :`LocalExposureHighlightContrastScale` _contrast :`LocalExposureShadowContrastScale` _contrast)
      (bind _returnvalue_2 (`GameplayStatics.GetActorOfClass` "/Game/FirstPerson/Blueprints/BP_FirstPersonCharacter.BP_FirstPersonCharacter_C"))
      (`CameraComponent.SetFieldOfView` (`/Game/FirstPerson/Blueprints/BP_FirstPersonCharacter.FirstPersonCamera` _returnvalue_2) (`KismetMathLibrary.Conv_IntToDouble` (`/Game/SaveGame/BP_SaveGame.FOV` `BP Save`))))))

(fn `SetSanityLevels`
  (bind _maxsanity (`self.MaxSanity`))
  (set `self.Sanity90` (`KismetMathLibrary.FTrunc` (* _maxsanity 0.9)))
  (set `self.Sanity80` (`KismetMathLibrary.FTrunc` (* _maxsanity 0.8)))
  (set `self.Sanity70` (`KismetMathLibrary.FTrunc` (* _maxsanity 0.7)))
  (set `self.Sanity60` (`KismetMathLibrary.FTrunc` (* _maxsanity 0.6)))
  (set `self.Sanity50` (`KismetMathLibrary.FTrunc` (* _maxsanity 0.5)))
  (set `self.Sanity40` (`KismetMathLibrary.FTrunc` (* _maxsanity 0.4)))
  (set `self.Sanity30` (`KismetMathLibrary.FTrunc` (* _maxsanity 0.3)))
  (set `self.Sanity20` (`KismetMathLibrary.FTrunc` (* _maxsanity 0.2)))
  (set `self.Sanity10` (`KismetMathLibrary.FTrunc` (* _maxsanity 0.1))))

(fn `UserConstructionScript`)