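; Printer task actor that is activated by a game state event when the current day matches its DayToActivate.
; A one-time interaction recursively reveals each "Paper"-tagged component, sliding it forward on a timeline with printer sound.
; When printing ends, the task deactivates and Paper overlaps are enabled, allowing a single grab.
; Grabbing spawns a physics BP_Paper into the player's physics handle and hides the printed sheets.
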(event `self.ReceiveBeginPlay`
  (bind _returnvalue (`GameplayStatics.GetActorOfClass` "/Game/Menu/BP_MyGameState.BP_MyGameState_C"))
  (add `/Game/Menu/BP_MyGameState.ActivateTasks` _returnvalue (delegate `Activate Task`)))

(event `Activate Task`
  (bind _returnvalue (`GameplayStatics.GetActorOfClass` "/Game/Menu/BP_MyGameState.BP_MyGameState_C"))
  (bind _output_get (set `self.Gamestate` _returnvalue))
  (if (== (`/Game/Menu/BP_MyGameState.CurrentDay` _output_get) (`self.Day To Activate`))
    (set `self.Task Activated` true)
    (else
      (set `self.Task Activated` false))))

(event `/Game/Tasks/Interfaces/BPI_Interactable.OnInteract`
  (params (InteractingPlayer :type "/Game/FirstPerson/Blueprints/BP_FirstPersonCharacter Object Reference"))
  (if (`self.Task Activated`)
    (`/Engine/EditorBlueprintResources/StandardMacros.DoOnce` false
      (:`Completed`
        (set `self.Papers` (`self.GetComponentsByTag` "/Script/Engine.PrimitiveComponent" "Paper"))
        (`self.Print`)))))

(event `Print`
  (bind _papers (`self.Papers`))
  (bind _output (`|GetArrayItem` _papers))
  (`|ExecutionSequence`
    (:`then_0`
      (if (> (`KismetArrayLibrary.Array_Length` _papers) 0)
        (`KismetSystemLibrary.Delay` (`self.Delay`))
        (`SceneComponent.SetHiddenInGame` _output false false)
        (`Timeline|Timeline` :!via `PlayFromStart`
          (:`Update`
            (`SceneComponent.K2_SetWorldLocation` _output (+ (`SceneComponent.K2_GetComponentLocation` _output) (`SceneComponent.GetForwardVector` _output)) false false))
          (:`Finished`
            (`KismetArrayLibrary.Array_RemoveItem` (`self.Papers`) _output)
            (`|ExecutionSequence`
              (:`then_0`
                (`/Engine/EditorBlueprintResources/StandardMacros.DoOnce` false
                  (:`Completed`
                    (set `self.Delay` 1.0))))
              (:`then_1`
                (`self.Print`)))))
        (else
          (set `PrimitiveComponent.bGenerateOverlapEvents` true (`self.Paper`))
          (set `self.Task Activated` false))))
    (:`then_1`
      (`GameplayStatics.PlaySoundAtLocation` "/Game/Sound/Printer/Printer_Sound_A02.Printer_Sound_A02" (`self.K2_GetActorLocation`) (struct) 1.0 1.0 0.0 "/Game/Sound/Printer/PrinterSoundAttenuation.PrinterSoundAttenuation" null null null))))

(event `/Game/Tasks/Interfaces/BPI_Grabbable.OnGrab`
  (params (`Interacting Player` :type "/Game/FirstPerson/Blueprints/BP_FirstPersonCharacter Object Reference"))
  (if (`PrimitiveComponent.bGenerateOverlapEvents` (`self.Paper`))
    (`/Engine/EditorBlueprintResources/StandardMacros.DoOnce` false
      (:`Completed`
        (bind _returnvalue (`|SpawnActorFromClass` "/Game/Tasks/Printing/BP_Paper.BP_Paper_C" (`KismetMathLibrary.MakeTransform` (`SceneComponent.K2_GetComponentLocation` (`self.Plane`))) "AlwaysSpawn" "MultiplyWithRoot" null null))
        (set `/Game/FirstPerson/Blueprints/BP_FirstPersonCharacter.HeldObject` _returnvalue `Interacting Player`)
        (bind _paper (`/Game/Tasks/Printing/BP_Paper.Paper` _returnvalue))
        (`PrimitiveComponent.SetSimulatePhysics` _paper true)
        (`PhysicsHandleComponent.GrabComponentAtLocationWithRotation` (`/Game/FirstPerson/Blueprints/BP_FirstPersonCharacter.PhysicsHandle` `Interacting Player`) _paper "None" (`SceneComponent.K2_GetComponentLocation` _paper) (`SceneComponent.K2_GetComponentRotation` _paper))
        (`SceneComponent.SetHiddenInGame` (`self.GetComponentsByTag` "/Script/Engine.PrimitiveComponent" "Paper") true false)))))

(fn `CheckActivated`
  (returns (isActivated :type Boolean))
  (return (`self.Task Activated`)))

(fn `TaskDescription`
  (returns (Description :type Text))
  (return (`self.Description`)))

(fn `UserConstructionScript`)