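; BP_Table is an interactable table where a player sets down the object they are holding.
; On interact, it releases a valid HeldObject from the player's PhysicsHandle and turns off physics on its primitive components tagged "xxx".
; It then teleports the object to the DropZone's location and rotation, sends it OnReleaseMessage and clears the player's reference.
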(event `/Game/Tasks/BPI_Interactable.OnInteract`
  (params (InteractingPlayer :type "/Game/FirstPerson/Blueprints/BP_FirstPersonCharacter Object Reference"))
  (bind _dropzone (`self.DropZone`))
  (bind _heldobject (`/Game/FirstPerson/Blueprints/BP_FirstPersonCharacter.HeldObject` InteractingPlayer))
  (`/Engine/EditorBlueprintResources/StandardMacros.IsValid` _heldobject
    (:`Is Valid`
      (`PhysicsHandleComponent.ReleaseComponent` (`/Game/FirstPerson/Blueprints/BP_FirstPersonCharacter.PhysicsHandle` InteractingPlayer))
      (`PrimitiveComponent.SetSimulatePhysics` (`self.GetComponentsByTag` _heldobject "/Script/Engine.PrimitiveComponent" "xxx") false)
      (`self.K2_SetActorLocationAndRotation` _heldobject (`SceneComponent.K2_GetComponentLocation` _dropzone) (`SceneComponent.K2_GetComponentRotation` _dropzone) false true)
      (message `/Game/Tasks/BPI_Grabbable.OnRelease` _heldobject)
      (set `/Game/FirstPerson/Blueprints/BP_FirstPersonCharacter.HeldObject` null InteractingPlayer))))

(fn `UserConstructionScript`)