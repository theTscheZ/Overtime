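; Interactable drawer task in which the player sorts files alphabetically to gain sanity.
; Interacting slides the drawer via a timeline and enables the player's raycast, which the trigger box also toggles.
; ShowName briefly displays a tagged folder's object name; picks append that text to an order list, clearing it on an alphabetical mistake.
; Completion closes the drawer and deactivates the task, while Tick turns both text renders with the player's mesh.
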(event `self.ReceiveBeginPlay`
  (bind _returnvalue (`GameplayStatics.GetActorOfClass` "/Game/FirstPerson/Blueprints/BP_FirstPersonCharacter.BP_FirstPersonCharacter_C"))
  (set `self.Player` _returnvalue)
  (bind _returnvalue_2 (`GameplayStatics.GetActorOfClass` "/Game/Menu/BP_MyGameState.BP_MyGameState_C"))
  (set `self.GameState` _returnvalue_2))

(event `self.ReceiveTick`
  (params (DeltaSeconds :type "Float (single-precision)"))
  (bind _textrender1 (`self.TextRender1`))
  (bind _textrender (`self.TextRender`))
  (bind (_returnvalue_roll _returnvalue_pitch _returnvalue_yaw) (`KismetMathLibrary.BreakRotator` (`SceneComponent.K2_GetComponentRotation` (`Character.Mesh` (`GameplayStatics.GetPlayerCharacter` 0)))))
  (bind _returnvalue (+ _returnvalue_yaw 180.0))
  (`/Engine/EditorBlueprintResources/StandardMacros.IsValid` _textrender
    (:`Is Valid`
      (`SceneComponent.K2_SetWorldRotation` _textrender (`KismetMathLibrary.MakeRotator` _returnvalue_roll _returnvalue_pitch _returnvalue) false false)
      (`/Engine/EditorBlueprintResources/StandardMacros.IsValid` _textrender1
        (:`Is Valid`
          (`SceneComponent.K2_SetWorldRotation` _textrender1 (`KismetMathLibrary.MakeRotator` _returnvalue_roll _returnvalue_pitch _returnvalue) false false))))))

(event `self.OnInteract`
  (params (InteractingPlayer :type "/Game/FirstPerson/Blueprints/BP_FirstPersonCharacter Object Reference"))
  (bind _textrender1 (`self.TextRender1`))
  (bind _order (`self.Order`))
  (bind _drawer (`self.Drawer`))
  (bind _returnvalue (`KismetTextLibrary.Conv_TextToString` (`TextRenderComponent.Text` (`self.TextRender`))))
  (if (`self.Task Activated`)
    (`|ExecutionSequence`
      (:`then_0`
        (`/Engine/EditorBlueprintResources/StandardMacros.DoOnce` false
          (:`Completed`
            (`Timeline|Timeline` :!via `PlayFromStart` :!label _label
              (:`Update`
                (`SceneComponent.K2_SetWorldLocation` _drawer (+ (`SceneComponent.K2_GetComponentLocation` _drawer) (* (`SceneComponent.GetForwardVector` _drawer) (`self.Direction`))) false false))
              (:`Finished`
                (`/Engine/EditorBlueprintResources/StandardMacros.DoOnce` false
                  (:`Completed`
                    (set `self.Direction` (* (`self.Direction`) -1))
                    (set `self.hasTaskStarted` true)
                    (set `/Game/FirstPerson/Blueprints/BP_FirstPersonCharacter.isRayCastEnabled` true (`self.Player`))
                    (goto _label_2 :!via `Reset`))))))))
      (:`then_1`
        (`/Engine/EditorBlueprintResources/StandardMacros.DoOnce` true :!label _label_2
          (:`Completed`
            (bind _returnvalue_2 (`KismetArrayLibrary.Array_Add` (`self.Order`) _returnvalue))
            (`TextRenderComponent.K2_SetText` _textrender1 (`KismetTextLibrary.Conv_StringToText` (`KismetStringLibrary.Concat_StrStr` (`KismetTextLibrary.Conv_TextToString` (`TextRenderComponent.Text` _textrender1)) _returnvalue)))
            (if (`KismetMathLibrary.Conv_IntToBool` _returnvalue_2)
              (if (`/Game/BP_FunctionLibrary1.Is String A Less Than String B` (`|GetArrayItem` _order (- _returnvalue_2 1)) (`|GetArrayItem` _order _returnvalue_2))
                (for (_ _array_index) (`self.Order`)
                  _)
                (if (== _array_index (`self.OrdnerCount`))
                  (set `/Game/FirstPerson/Blueprints/BP_FirstPersonCharacter.isRayCastEnabled` false (`self.Player`))
                  (set `self.hasTaskStarted` false)
                  (`/Game/Menu/BP_MyGameState.AddSanity` (`self.GameState`) (`self.GainableSanity`))
                  (set `self.Task Activated` false)
                  (goto _label :!via `PlayFromStart`)
                  (else
                    (goto _label_2 :!via `Reset`)))
                (else
                  (`KismetArrayLibrary.Array_Clear` (`self.Order`))
                  (`TextRenderComponent.K2_SetText` (`self.TextRender1`) (`KismetTextLibrary.GetEmptyText`))
                  (goto _label_2 :!via `Reset`)))
              (else
                (goto _label_2 :!via `Reset`)))))))))

(event `Show Name`
  (params (Component :type "PrimitiveComponent Object Reference"))
  (bind _textrender (`self.TextRender`))
  (if (`ActorComponent.ComponentHasTag` Component "Folder")
    (`TextRenderComponent.K2_SetText` _textrender (`KismetTextLibrary.Conv_StringToText` (`KismetSystemLibrary.GetObjectName` Component)))
    (`KismetSystemLibrary.Delay` 0.2)
    (`TextRenderComponent.K2_SetText` _textrender (`KismetTextLibrary.GetEmptyText`))))

(event `self.Box.OnComponentBeginOverlap`
  (params (OverlappedComponent :type "PrimitiveComponent Object Reference") (OtherActor :type "Actor Object Reference") (OtherComp :type "PrimitiveComponent Object Reference") (OtherBodyIndex :type Integer) (bFromSweep :type Boolean) (SweepResult :type "HitResult Structure (by ref)"))
  (if (`self.hasTaskStarted`)
    (bind _asbp_first_person_character (cast `/Game/FirstPerson/Blueprints/BP_FirstPersonCharacter` OtherActor))
    (set `/Game/FirstPerson/Blueprints/BP_FirstPersonCharacter.isRayCastEnabled` true _asbp_first_person_character)))

(event `self.Box.OnComponentEndOverlap`
  (params (OverlappedComponent :type "PrimitiveComponent Object Reference") (OtherActor :type "Actor Object Reference") (OtherComp :type "PrimitiveComponent Object Reference") (OtherBodyIndex :type Integer))
  (bind _asbp_first_person_character (cast `/Game/FirstPerson/Blueprints/BP_FirstPersonCharacter` OtherActor))
  (set `/Game/FirstPerson/Blueprints/BP_FirstPersonCharacter.isRayCastEnabled` false _asbp_first_person_character))

(fn `CheckActivated`
  (returns (isActivated :type Boolean))
  (return (`self.Task Activated`)))

(fn `TaskDescription`
  (returns (Description :type Text))
  (return "Sortiere die Akten alphabetisch"))

(fn `UserConstructionScript`)